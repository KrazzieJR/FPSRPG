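; Player character Blueprint for an FPS RPG, handling first-person movement, shooting, XP leveling and UI.
; On BeginPlay it attaches a spawned gun to the camera, creates the HUD and hidden menu, registers with the game instance and loads the saved level.
; Leveling doubles the XP requirement and boosts walk speed and acceleration; a debug key forces it.
; The menu input toggles UI and input mode; SmokeScreen and FireBall abilities only print placeholders.
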(event `self.ReceiveBeginPlay`
  (bind (_returnvalue_location _returnvalue_rotation _returnvalue_scale) (`KismetMathLibrary.BreakTransform` (`SceneComponent.K2_GetComponentToWorld` (`self.Camera`))))
  ;[1 1 1] BeginPlay
  (bind _returnvalue (`|SpawnActorFromClass` "/Game/CustomContent/Guns/BaseGun.BaseGun_C" (`KismetMathLibrary.MakeTransform` (+ _returnvalue_location (* (`KismetMathLibrary.GetForwardVector` _returnvalue_rotation) 100.0) (0.0 50.0 -20.0)) (`KismetMathLibrary.MakeRotator` (.roll _returnvalue_rotation) (.pitch _returnvalue_rotation) (+ (.yaw _returnvalue_rotation) 180.0)) _returnvalue_scale) "Undefined" "OverrideRootScale" null self null))
  (bind _output_get (set `self.CurrentGun` _returnvalue))
  (`self.K2_AttachToComponent` _output_get (`self.Camera`) "None" "KeepWorld" "KeepWorld" "KeepWorld" true)
  (`self.CreateHud`)
  (`self.CreatePlayerMenu`)
  (bind _asfpsrpggame_instance (cast `/Game/CustomContent/FPSRPGGameInstance` (`GameplayStatics.GetGameInstance`)))
  (set `/Game/CustomContent/FPSRPGGameInstance.PlayerRef` self _asfpsrpggame_instance)
  (bind _asrpgfpssave_game (cast `/Game/CustomContent/RPGFPSSaveGame` (`/Game/CustomContent/FPSRPGGameInstance.CurrentSave` _asfpsrpggame_instance)))
  (set `self.Level` (`/Game/CustomContent/RPGFPSSaveGame.PlayerLevel` _asrpgfpssave_game)))

(event `InputAxis|LookRight`
  (params (AxisValue :type "Float (single-precision)"))
  ;[1 0.8794 0.2077] Movement
  (`self.AddControllerYawInput` AxisValue))

(event `InputAction|Shoot`
  (params (Key :type "Key Structure"))
  (bind _currentgun (`self.CurrentGun`))
  ;[1 0.03977 0.009923] Shoot
  (:`Pressed`
    (`/Game/CustomContent/Guns/BaseGun.Shoot` _currentgun)
    (`/Game/CustomContent/Guns/BaseGun.StartShooting` _currentgun))
  (:`Released`
    (`/Game/CustomContent/Guns/BaseGun.StopShooting` _currentgun)))

(event `InputAxis|LookUp`
  (params (AxisValue :type "Float (single-precision)"))
  ;[1 0.8794 0.2077] Movement
  (`self.AddControllerPitchInput` AxisValue))

(event `InputAxis|MoveRight`
  (params (AxisValue :type "Float (single-precision)"))
  ;[1 0.8794 0.2077] Movement
  (`self.AddMovementInput` (`self.GetActorRightVector`) AxisValue true))

(event `UpdateXP`
  (params (XP :type Integer))
  ;[0.09797 0.0904 1] UpdateXP
  (set `self.CurrentXP` (+ XP (`self.CurrentXP`)))
  (if (>= (`self.CurrentXP`) (`self.XPNeededForThisLevel`))
    (`self.LevelUp`)))

(event `InputAxis|MoveForward`
  (params (AxisValue :type "Float (single-precision)"))
  ;[1 0.8794 0.2077] Movement
  (`self.AddMovementInput` (`self.GetActorForwardVector`) AxisValue))

(event `InputAction|Jump`
  (params (Key :type "Key Structure"))
  ;[1 0.8794 0.2077] Movement
  (:`Pressed`
    (`self.Jump`))
  (:`Released`
    (`self.StopJumping`)))

(event `LevelUp`
  ;[0.1295 1 0.1096] LevelUP
  (`self.UpdateLevel`)
  (`self.UpdateMovement`))

(event `Key|P`
  (params (Key :type "Key Structure"))
  ;[1 1 1] Debug
  (:`Pressed`
    (set `self.CurrentXP` (`self.XPNeededForThisLevel`))
    (`self.LevelUp`)))

(event `InputAction|OpenMenu`
  (params (Key :type "Key Structure"))
  (bind _returnvalue (`GameplayStatics.GetPlayerController` 0))
  (bind _hudref (`self.HUDRef`))
  (bind _menuref (`self.MenuRef`))
  (:`Pressed`
    (`/Engine/EditorBlueprintResources/StandardMacros.FlipFlop`
      (:`A`
        (`Widget.SetVisibility` _hudref "Hidden")
        (`Widget.SetVisibility` _menuref "Visible")
        (set `PlayerController.bShowMouseCursor` true _returnvalue)
        (`WidgetBlueprintLibrary.SetInputMode_GameAndUIEx` _returnvalue _menuref "DoNotLock" false))
      (:`B`
        (`Widget.SetVisibility` _hudref "Visible")
        (`Widget.SetVisibility` _menuref "Hidden")
        (set `PlayerController.bShowMouseCursor` false _returnvalue)
        (`WidgetBlueprintLibrary.SetInputMode_GameOnly` _returnvalue)))))

(fn `Abilities`
  (params (Ability :type "/Game/CustomContent/Abilities Enum" :default "NewEnumerator0"))
  (switch `/Game/CustomContent/Abilities` Ability
    (:`NewEnumerator0`
      (`self.SmokeScreen`)
      (return))
    (:`NewEnumerator1`
      (`self.FireBall`))))

(fn `CreateHud`
  (bind _returnvalue (`|CreateWidget` "/Game/CustomContent/UI_Stuff/PlayerHUD.PlayerHUD_C" null self))
  (bind _output_get (set `self.HUDRef` _returnvalue))
  (`UserWidget.AddToViewport` _output_get 0))

(fn `CreatePlayerMenu`
  (bind _returnvalue (`|CreateWidget` "/Game/CustomContent/UI_Stuff/PlayerMenu.PlayerMenu_C" null self))
  (set `self.MenuRef` _returnvalue)
  (`UserWidget.AddToViewport` _returnvalue 0)
  (`Widget.SetVisibility` _returnvalue "Hidden"))

(fn `FireBall`
  (`KismetSystemLibrary.PrintString` "FireBall"))

(fn `SmokeScreen`
  (`KismetSystemLibrary.PrintString` "SmokeScreen"))

(fn `UpdateLevel`
  (bind _xpneededforthislevel (`self.XPNeededForThisLevel`))
  (`/Engine/EditorBlueprintResources/StandardMacros.IncrementInt` (`self.Level`)
    (:`  `
      (set `self.CurrentXP` (- (`self.CurrentXP`) _xpneededforthislevel))
      (set `self.XPNeededForThisLevel` (* _xpneededforthislevel 2)))))

(fn `UpdateMovement`
  (bind _charactermovement (`self.CharacterMovement`))
  (bind _returnvalue (`CharacterMovementComponent.GetMaxAcceleration` _charactermovement))
  (bind _maxwalkspeed (`CharacterMovementComponent.MaxWalkSpeed` _charactermovement))
  (set `CharacterMovementComponent.MaxWalkSpeed` (+ _maxwalkspeed (* _maxwalkspeed (`self.MoveSpeedModifier`))) _charactermovement)
  (set `CharacterMovementComponent.MaxAcceleration` (+ _returnvalue (* _returnvalue (`self.MoveSpeedModifier`))) _charactermovement))

(fn `UserConstructionScript`)